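; Game mode for a platformer that manages score, pause, player respawn and level completion.
; On BeginPlay it builds the game UI, caches the PlayerStart transform and all checkpoints, then clears the game instance's loading-from-save flag.
; Pausing pushes or clears a menu on a UI widget stack; death and finish use camera fades before respawning or opening EndScreen.
; CheckpointTeleport cycles through checkpoint arrow transforms, wrapping around.
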(event `self.ReceiveBeginPlay`
  (`self.Init UI`)
  (`self.Setup Spawnpoint`)
  (`self.Get Checkpoints`)
  (`self.Input Mode`)
  (`KismetSystemLibrary.Delay` 0.2)
  (bind _asgi_plattformer (cast `/Game/Blueprints/GI_Plattformer` (`GameplayStatics.GetGameInstance`)))
  (set `/Game/Blueprints/GI_Plattformer.Loading from Save` false _asgi_plattformer))

(event `AddScore`
  (params (Value :type Integer))
  (bind _output_get (set `self.Score` (+ Value (`self.Score`))))
  (`/Game/Assets/UI-HUD/WBP_GameUI.UpdateScore` (`self.GameUI`) _output_get))

(event `Input Mode`
  (`WidgetBlueprintLibrary.SetInputMode_GameOnly` (`GameplayStatics.GetPlayerController` 0)))

(event `Init UI`
  (bind _returnvalue (`|CreateWidget` "/Game/Assets/UI-HUD/WBP_GameUI.WBP_GameUI_C"))
  (bind _output_get (set `self.GameUI` _returnvalue))
  (`UserWidget.AddToViewport` _output_get 0)
  (`CommonActivatableWidgetContainerBase.BP_AddWidget` (`/Game/Assets/UI-HUD/WBP_GameUI.GameplayStack` _output_get) "/Game/Assets/UI-HUD/WBP_GameplayUI.WBP_GameplayUI_C"))

(event `PauseGame`
  (bind _returnvalue (`GameplayStatics.GetPlayerController` 0))
  ;[1 1 1] Pause/Unpause
  (`CommonActivatableWidgetContainerBase.BP_AddWidget` (`/Game/Assets/UI-HUD/WBP_GameUI.PauseStack` (`self.GameUI`)) "/Game/Assets/UI-HUD/WBP_PauseMenu.WBP_PauseMenu_C")
  (`GameplayStatics.SetGamePaused` true)
  (`WidgetBlueprintLibrary.SetInputMode_UIOnlyEx` _returnvalue null)
  (set `PlayerController.bShowMouseCursor` true _returnvalue))

(event `UnPauseGame`
  (bind _returnvalue (`GameplayStatics.GetPlayerController` 0))
  ;[1 1 1] Pause/Unpause
  (`CommonActivatableWidgetContainerBase.ClearWidgets` (`/Game/Assets/UI-HUD/WBP_GameUI.PauseStack` (`self.GameUI`)))
  (`GameplayStatics.SetGamePaused` false)
  (`WidgetBlueprintLibrary.SetInputMode_GameOnly` _returnvalue)
  (set `PlayerController.bShowMouseCursor` false _returnvalue))

(event `PlayerDied`
  (`PlayerCameraManager.StartCameraFade` (`GameplayStatics.GetPlayerCameraManager` 0) 0.0 1.0 1.0 (struct :`A` 1.0) false true)
  (`KismetSystemLibrary.Delay` 1.0)
  (`self.PlayerSpawn`))

(event `Get Checkpoints`
  (bind _outactors (`GameplayStatics.GetAllActorsOfClass` "/Game/Blueprints/Actor/BP_Checkpoint.BP_Checkpoint_C"))
  (set `self.Checkpoints` _outactors))

(event `PlayerSpawn`
  (bind _player_spawnpoint (`self.Player Spawnpoint`))
  (bind _returnvalue (`|SpawnActorFromClass` "/Game/Blueprints/BP_Player.BP_Player_C" (`KismetMathLibrary.MakeTransform` (.location _player_spawnpoint) (`KismetMathLibrary.MakeRotator` 0.0 0.0 (.yaw (.rotation _player_spawnpoint)))) "Undefined" "OverrideRootScale" null null))
  (`Controller.Possess` (`GameplayStatics.GetPlayerController` 0) _returnvalue)
  (`PlayerCameraManager.StartCameraFade` (`GameplayStatics.GetPlayerCameraManager` 0) 1.0 0.0 1.0 (struct :`A` 1.0) false true))

(event `Setup Spawnpoint`
  (bind _returnvalue (`GameplayStatics.GetActorOfClass` "/Script/Engine.PlayerStart"))
  (set `self.Player Spawnpoint` (`self.GetTransform` _returnvalue)))

(event `FinishGame`
  (`PlayerCameraManager.StartCameraFade` :`self` (`GameplayStatics.GetPlayerCameraManager` 0) :`ToAlpha` 1.0 :`Duration` 2.0 :`bHoldWhenFinished` true)
  (`KismetSystemLibrary.Delay` 2.0)
  (`GameplayStatics.OpenLevel` "EndScreen"))

(fn `CheckpointTeleport`
  (returns (`new Transform` :type "Transform Structure"))
  (locals (NextTransform :type "Transform Structure"))
  (set `local.NextTransform` (`SceneComponent.K2_GetComponentToWorld` (`/Game/Blueprints/Actor/BP_Checkpoint.Arrow` (`|GetArrayItem` (`self.Checkpoints`) (`self.Checkpointindex`)))))
  (bind _output_get (set `self.Checkpointindex` (+ (`self.Checkpointindex`) 1)))
  (if (== _output_get (`KismetArrayLibrary.Array_Length` (`self.Checkpoints`)))
    (set `self.Checkpointindex` 0))
  (return (`local.NextTransform`)))

(fn `UserConstructionScript`)