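; Game instance for a platformer that owns the save object and handles resetting, saving and loading progress in a single slot.
; Init creates a fresh save object, and saving stores the player's transform, control rotation and current level name before writing to disk.
; Loading restores the save object, sets a LoadingFromSave flag and opens the saved level, without applying the player transform itself.
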(event `self.ReceiveInit`
  (`self.ResetGame`))

(event `ResetGame`
  (bind _returnvalue (`GameplayStatics.CreateSaveGameObject` "/Game/Blueprints/BP_SaveGame.BP_SaveGame_C"))
  (set `self.Save Game Ref` _returnvalue)
  (set `self.Loading from Save` false))

(event `Save Game`
  (bind _save_game_ref (`self.Save Game Ref`))
  (`|ExecutionSequence`
    (:`then_0`
      (bind _returnvalue (`GameplayStatics.GetActorOfClass` "/Game/Blueprints/BP_Player.BP_Player_C"))
      (set `/Game/Blueprints/BP_SaveGame.PlayerTransform` (`Actor.GetTransform` _returnvalue) _save_game_ref)
      (set `/Game/Blueprints/BP_SaveGame.Player Camera Rot` (`Pawn.GetControlRotation` _returnvalue) _save_game_ref))
    (:`then_1`
      (bind _returnvalue_2 (`GameplayStatics.GetCurrentLevelName` true))
      (set `/Game/Blueprints/BP_SaveGame.CurrentLevel` _returnvalue_2 (`self.Save Game Ref`)))
    (:`then_5`
      (bind _returnvalue_3 (`GameplayStatics.SaveGameToSlot` (`self.Save Game Ref`) (`self.Slot Name`)))
      (if _returnvalue_3
        (`KismetSystemLibrary.PrintString` "Save Success")
        (else
          (`KismetSystemLibrary.PrintString` "Save FAILED"))))))

(event `Load Game`
  (bind _returnvalue (`GameplayStatics.DoesSaveGameExist` (`self.Slot Name`)))
  (if _returnvalue
    (set `self.Loading from Save` true)
    (bind _returnvalue_2 (`GameplayStatics.LoadGameFromSlot` (`self.Slot Name`)))
    (bind _asbp_save_game (cast `/Game/Blueprints/BP_SaveGame` _returnvalue_2))
    (bind _output_get (set `self.Save Game Ref` _asbp_save_game))
    (`GameplayStatics.OpenLevel` (`KismetStringLibrary.Conv_StringToName` (`/Game/Blueprints/BP_SaveGame.CurrentLevel` _output_get)))
    (else
      (`KismetSystemLibrary.PrintString` "No Saved Game"))))