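; Pressure plate actor that the player steps on to switch other actors on and off.
; Player overlap plays a timeline that lowers the plate mesh, and leaving reverses it.
; When fully pressed, it plays an optional level sequence once and sends an on message through BPI_Trigger to each implementing actor in ActorsToTrigger.
; When fully released, it sends those actors the off message.
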(event `self.Collision.OnComponentBeginOverlap`
  (params (OverlappedComponent :type "PrimitiveComponent Object Reference") (OtherActor :type "Actor Object Reference") (OtherComp :type "PrimitiveComponent Object Reference") (OtherBodyIndex :type Integer) (bFromSweep :type Boolean) (SweepResult :type "HitResult Structure (by ref)"))
  (bind _levelsequence (`self.LevelSequence`))
  (cast `/Game/Blueprints/BP_Player` OtherActor)
  (bind (_direction _alpha) (`Timeline|ButtonAnim` :!label _label)
    (:`Update`
      (`SceneComponent.K2_SetRelativeLocation` (`self.BP_Plate`) (`KismetMathLibrary.VLerp` (0.0 0.0 0.0) (0.0 0.0 -6.0) _alpha) false false))
    (:`Finished`
      (switch `ETimelineDirection` _direction
        (:`Forward`
          (`|ExecutionSequence`
            (:`then_0`
              ;[1 1 1] Player LevelSequence
              (`/Engine/EditorBlueprintResources/StandardMacros.DoOnce` false
                (:`Completed`
                  (`/Engine/EditorBlueprintResources/StandardMacros.IsValid` _levelsequence
                    (:`Is Valid`
                      (`MovieSceneSequencePlayer.Play` (`LevelSequenceActor.SequencePlayer` _levelsequence)))))))
            (:`then_1`
              ;[1 1 1] Actors to Trigger Loop On
              (for _array_element (`self.ActorsToTrigger`)
                (if (`KismetSystemLibrary.DoesImplementInterface` _array_element "/Game/Blueprints/Interfaces/BPI_Trigger.BPI_Trigger_C")
                  (message `/Game/Blueprints/Interfaces/BPI_Trigger.Trigger` _array_element true null))))))
        (:`Backward`
          ;[1 1 1] Actors to Trigger Loop Off
          (for _array_element_2 (`self.ActorsToTrigger`)
            (if (`KismetSystemLibrary.DoesImplementInterface` _array_element_2 "/Game/Blueprints/Interfaces/BPI_Trigger.BPI_Trigger_C")
              (message `/Game/Blueprints/Interfaces/BPI_Trigger.Trigger` _array_element_2 false null))))))))

(event `self.Collision.OnComponentEndOverlap`
  (params (OverlappedComponent :type "PrimitiveComponent Object Reference") (OtherActor :type "Actor Object Reference") (OtherComp :type "PrimitiveComponent Object Reference") (OtherBodyIndex :type Integer))
  (cast `/Game/Blueprints/BP_Player` OtherActor)
  (goto _label :!via `Reverse`))

(fn `UserConstructionScript`)