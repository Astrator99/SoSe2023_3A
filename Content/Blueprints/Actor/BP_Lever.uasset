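; Lever actor that the player interacts with to toggle on and off, signaling linked trigger targets.
; Interacting plays or reverses a timeline that lerps the lever's rotation between start and end.
; On finish, the timeline direction sets IsOn, which is sent to each target implementing BPI_Trigger.
; An optional level sequence plays only the first time the animation finishes.
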(event `self.ReceiveBeginPlay`)

(event `Interacted`
  (bind _levelsequence (`self.LevelSequence`))
  (if (not (`self.IsOn`))
    (bind (_direction _alpha) (`Timeline|LeverAnim` :!label _label)
      (:`Update`
        (`SceneComponent.K2_SetRelativeRotation` (`self.Lever`) (`KismetMathLibrary.RLerp` (`self.Start Rotation`) (`self.End Rotation`) _alpha) false false))
      (:`Finished`
        (`|ExecutionSequence`
          (:`then_0`
            (set `self.IsOn` (select `ETimelineDirection` _direction :`Forward` true)))
          (:`then_1`
            ;[1 1 1] Actors to Trigger Loop
            (for _array_element (`self.TriggerTarget`)
              (if (`KismetSystemLibrary.DoesImplementInterface` _array_element "/Game/Blueprints/Interfaces/BPI_Trigger.BPI_Trigger_C")
                (message `/Game/Blueprints/Interfaces/BPI_Trigger.Trigger` _array_element (`self.IsOn`) self))))
          (:`then_2`
            ;[1 1 1] Player LevelSequence
            (`/Engine/EditorBlueprintResources/StandardMacros.DoOnce` false
              (:`Completed`
                (`/Engine/EditorBlueprintResources/StandardMacros.IsValid` _levelsequence
                  (:`Is Valid`
                    (`MovieSceneSequencePlayer.Play` (`LevelSequenceActor.SequencePlayer` _levelsequence))))))))))
    (else
      (goto _label :!via `Reverse`))))

(event `/Game/Blueprints/Interfaces/BPI_Interactable.Interact`
  (`self.Interacted`))

(fn `UserConstructionScript`)