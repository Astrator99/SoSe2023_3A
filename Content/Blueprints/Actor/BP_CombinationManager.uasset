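; Puzzle manager actor that fires a one-time response when the wanted combination of actors is switched on, in any order.
; Trigger events add or remove actors from CurrentCombination, which is checked against WantedCombination by length and membership.
; A match passes a DoOnce, sends TriggerMessage through BPI_Trigger to each implementing actor in ActorsToTrigger, then plays the LevelSequence if valid.
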(event `/Game/Blueprints/Interfaces/BPI_Trigger.Trigger`
  (params (On :type Boolean) (Actor :type "Actor Object Reference"))
  (bind _levelsequence (`self.LevelSequence`))
  (if On
    (`KismetArrayLibrary.Array_Add` (`self.Current Combination`) Actor)
    (if (== (`KismetArrayLibrary.Array_Length` (`self.Current Combination`)) (`KismetArrayLibrary.Array_Length` (`self.Wanted Combination`))) :!label _label
      (set `self.LoopBroken` false)
      (for _array_element (`self.Wanted Combination`) :!label _label_2
        (if (== (`KismetArrayLibrary.Array_Find` (`self.Current Combination`) _array_element) -1)
          (`self.BreakLoop`)
          (set `self.LoopBroken` true)))
      (if (not (`self.LoopBroken`))
        (`/Engine/EditorBlueprintResources/StandardMacros.DoOnce` false
          (:`Completed`
            (`|ExecutionSequence`
              (:`then_0`
                (for _array_element_2 (`self.ActorsToTrigger`)
                  (if (`KismetSystemLibrary.DoesImplementInterface` _array_element_2 "/Game/Blueprints/Interfaces/BPI_Trigger.BPI_Trigger_C")
                    (message `/Game/Blueprints/Interfaces/BPI_Trigger.Trigger` _array_element_2 true null))))
              (:`then_1`
                (`/Engine/EditorBlueprintResources/StandardMacros.IsValid` _levelsequence
                  (:`Is Valid`
                    (`MovieSceneSequencePlayer.Play` (`LevelSequenceActor.SequencePlayer` _levelsequence))))))))))
    (elif (!= (`KismetArrayLibrary.Array_Find` (`self.Current Combination`) Actor) -1)
      (`KismetArrayLibrary.Array_RemoveItem` (`self.Current Combination`) Actor)
      (goto _label))))

(event `BreakLoop`
  (goto _label_2 :!via `Break`))

(fn `UserConstructionScript`)