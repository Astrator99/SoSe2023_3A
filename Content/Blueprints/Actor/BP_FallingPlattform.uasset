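; Falling platform actor that disappears shortly after a Character steps on it and respawns after a delay.
; A box overlap, gated by DoOnce, waits a decay delay, then plays a scale timeline that drives the actor's scale.
; When the forward play finishes, collision and visibility are switched off.
; After the respawn delay both are restored, the timeline reverses, and the DoOnce resets for reuse.
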(event `self.Box.OnComponentBeginOverlap`
  (params (OverlappedComponent :type "PrimitiveComponent Object Reference") (OtherActor :type "Actor Object Reference") (OtherComp :type "PrimitiveComponent Object Reference") (OtherBodyIndex :type Integer) (bFromSweep :type Boolean) (SweepResult :type "HitResult Structure (by ref)"))
  (cast `Character` OtherActor)
  (`/Engine/EditorBlueprintResources/StandardMacros.DoOnce` false :!label _label
    (:`Completed`
      (`KismetSystemLibrary.Delay` (`self.Decay Delay`))
      (`self.Animate Plattform` false)
      (`KismetSystemLibrary.Delay` (`self.Respawn Delay`))
      (`self.Animate Plattform` true)
      (`self.Reset`))))

(event `Reset`
  (goto _label :!via `Reset`))

(event `Animate Plattform`
  (params (Visible :type Boolean))
  (if (not Visible)
    (bind (_direction _alpha) (`Timeline|ScaleAnim` :!label _label_2)
      (:`Update`
        (`self.SetActorScale3D` (`KismetMathLibrary.Conv_DoubleToVector` _alpha)))
      (:`Finished`
        (switch `ETimelineDirection` _direction
          (:`Forward`
            (`self.SetCollider` false)))))
    (else
      (`self.SetCollider` true)
      (goto _label_2 :!via `Reverse`))))

(event `SetCollider`
  (params (hasCollision :type Boolean))
  (`self.SetActorEnableCollision` hasCollision)
  (`self.SetActorHiddenInGame` (not hasCollision)))

(fn `UserConstructionScript`)