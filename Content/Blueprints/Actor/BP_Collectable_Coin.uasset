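; Collectable coin actor that animates in place and awards score when collected.
; On BeginPlay, the CoinTime timeline spins the mesh and bobs it vertically, and the coin's origin is stored.
; Collect plays a timeline that pulls the coin toward the collector while shrinking it, then adds Value to GM_Basic's score and destroys the coin.
; Collect has no caller in this graph, as the overlap event is disabled.
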(event `self.ReceiveBeginPlay`
  (`parent.ReceiveBeginPlay`)
  (`self.Animate`)
  (set `self.Coin Origin` (`self.K2_GetActorLocation`)))

(event `Animate`
  (bind (_direction _alpha _alphabounce) (`Timeline|CoinTime`)
    (:`Update`
      (`SceneComponent.K2_SetWorldRotation` (`self.StaticMesh`) (`KismetMathLibrary.RLerp` (struct) (struct :`Yaw` 360.0) _alpha) false false)
      (`SceneComponent.K2_SetRelativeLocation` (`self.StaticMesh`) (`KismetMathLibrary.VLerp` (0.0 0.0 -10.0) (0.0 0.0 10.0) _alphabounce) false false))))

(event `/Game/Blueprints/Interfaces/BPI_Collectable.Collect`
  (params (Collector :type "Pawn Object Reference"))
  ;[1 1 1] Suck in Coin Anim
  (bind (_direction _alpha) (`Timeline|CollectAnim`)
    (:`Update`
      (`self.K2_SetActorLocation` (`KismetMathLibrary.VLerp` (`self.Coin Origin`) (`self.K2_GetActorLocation` Collector) _alpha))
      (`self.SetActorScale3D` (`KismetMathLibrary.VLerp` (1.0 1.0 1.0) (0.0 0.0 0.0) _alpha)))
    (:`Finished`
      (bind _asgm_basic (cast `/Game/Blueprints/GM_Basic` (`GameplayStatics.GetGameMode`)))
      (`/Game/Blueprints/GM_Basic.AddScore` _asgm_basic (`self.Value`))
      (`self.K2_DestroyActor`))))

(fn `UserConstructionScript`
  (`parent.UserConstructionScript`))