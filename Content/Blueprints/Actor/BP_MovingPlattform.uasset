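; BP_MovingPlattform is a platform actor that travels along the spline of a referenced SplineBp actor.
; Each Tick, while AllowMove is set, it snaps to the world location at DistanceAlongSpline, then steps that distance by Speed and delta time.
; At an end it waits WaitTime before restarting (ClosedLoop) or reversing, or stops if OneWay without a loop.
; The Trigger event switches movement on or off.
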(event `self.ReceiveTick`
  (params (DeltaSeconds :type "Float (single-precision)"))
  (`self.MovePlattform`))

(event `Update Position`
  (`self.K2_SetActorLocation` (`SplineComponent.GetLocationAtDistanceAlongSpline` (`/Game/Blueprints/Actor/BP_Spline.Spline` (`self.Spline Bp`)) (`self.Distance Along Spline`) "World")))

(event `MovePlattform`
  (if (`self.Allow Move`)
    (`/Engine/EditorBlueprintResources/StandardMacros.IsValid` (`self.Spline Bp`)
      (:`Is Valid`
        (`|ExecutionSequence`
          (:`then_0`
            (`self.Update Position`))
          (:`then_1`
            (if (`self.MovingForward`)
              (if (< (`self.Distance Along Spline`) (`SplineComponent.GetSplineLength` (`/Game/Blueprints/Actor/BP_Spline.Spline` (`self.Spline Bp`))))
                ;[1 1 1] Count Distance Up
                (set `self.Distance Along Spline` (+ (`self.Distance Along Spline`) (* (`self.Speed`) (`GameplayStatics.GetWorldDeltaSeconds`))))
                (elif (`self.Closed Loop`)
                  (`KismetSystemLibrary.Delay` (`self.WaitTime`))
                  (set `self.Distance Along Spline` 0.0)
                  (elif (not (`self.OneWay`))
                    (`KismetSystemLibrary.Delay` (`self.WaitTime`))
                    (set `self.MovingForward` false))))
              (else
                ;[1 1 1] Plattform Move Backwards
                (if (> (`self.Distance Along Spline`) 0.0)
                  (set `self.Distance Along Spline` (- (`self.Distance Along Spline`) (* (`self.Speed`) (`GameplayStatics.GetWorldDeltaSeconds`))))
                  (elif (not (`self.OneWay`))
                    (`KismetSystemLibrary.Delay` (`self.WaitTime`))
                    (set `self.MovingForward` true)))))))))))

(event `/Game/Blueprints/Interfaces/BPI_Trigger.Trigger`
  (params (On :type Boolean) (Actor :type "Actor Object Reference"))
  (set `self.Allow Move` On))

(fn `UserConstructionScript`)