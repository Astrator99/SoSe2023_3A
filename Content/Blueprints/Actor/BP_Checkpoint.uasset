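; Checkpoint actor for a platformer that sets the player's respawn point and shows its active state with a Niagara effect.
; When BP_Player enters the capsule, it stores the Arrow transform in GM_Basic, switches off all registered checkpoints and activates itself.
; On BeginPlay, when loading from a save, it looks up its display name in the saved checkpoint map and, one tick later, restores that state and spawnpoint.
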(event `self.ReceiveBeginPlay`
  (`self.LoadCheckpoint`))

(event `self.Capsule.OnComponentBeginOverlap`
  (params (OverlappedComponent :type "PrimitiveComponent Object Reference") (OtherActor :type "Actor Object Reference") (OtherComp :type "PrimitiveComponent Object Reference") (OtherBodyIndex :type Integer) (bFromSweep :type Boolean) (SweepResult :type "HitResult Structure (by ref)"))
  (cast `/Game/Blueprints/BP_Player` OtherActor)
  (`ActorComponent.Activate` (`self.Niagara`) false)
  (bind _asgm_basic (cast `/Game/Blueprints/GM_Basic` (`GameplayStatics.GetGameMode`)))
  (set `/Game/Blueprints/GM_Basic.Player Spawnpoint` (`SceneComponent.K2_GetComponentToWorld` (`self.Arrow`)) _asgm_basic)
  (for _array_element (`/Game/Blueprints/GM_Basic.Checkpoints` _asgm_basic)
    (`ActorComponent.Deactivate` (`/Game/Blueprints/Actor/BP_Checkpoint.Niagara` _array_element))
    (set `/Game/Blueprints/Actor/BP_Checkpoint.isOn` false _array_element))
  (`ActorComponent.Activate` (`self.Niagara`) false)
  (set `self.isOn` true))

(event `LoadCheckpoint`
  (bind _asgi_plattformer (cast `/Game/Blueprints/GI_Plattformer` (`GameplayStatics.GetGameInstance`)))
  (if (`/Game/Blueprints/GI_Plattformer.Loading from Save` _asgi_plattformer)
    (if (`BlueprintMapLibrary.Map_Find` (`/Game/Blueprints/BP_SaveGame.Checkpoint` (`/Game/Blueprints/GI_Plattformer.Save Game Ref` _asgi_plattformer)) (`KismetSystemLibrary.GetDisplayName` self))
      (`KismetSystemLibrary.DelayUntilNextTick`)
      (`ActorComponent.Activate` (`self.Niagara`) false)
      (set `self.isOn` true)
      (bind _asgm_basic (cast `/Game/Blueprints/GM_Basic` (`GameplayStatics.GetGameMode`)))
      (set `/Game/Blueprints/GM_Basic.Player Spawnpoint` (`SceneComponent.K2_GetComponentToWorld` (`self.Arrow`)) _asgm_basic))))

(fn `UserConstructionScript`)